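; AI controller for enemies, running the Enemy_BT behavior tree and feeding it player sightings through the blackboard.
; On BeginPlay it starts the tree, caches the controlled Enemy_BP pawn and initializes the Direction key.
; AI perception updates for the player character set the CanSeePlayer key to whether the stimulus was sensed.
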(event `self.ReceiveBeginPlay`
  (`self.RunBehaviorTree` "/Game/Blueprints/AI/Enemy_BT.Enemy_BT")
  (bind _asenemy_bp (cast `/Game/Blueprints/AI/Enemy_BP` (`self.K2_GetPawn`)))
  (set `self.MyPawn` _asenemy_bp)
  (`BlackboardComponent.SetValueAsInt` (`AIBlueprintHelperLibrary.GetBlackboard` null) "Direction" 1))

(event `self.AIPerception.OnTargetPerceptionUpdated`
  (params (Actor :type "Actor Object Reference") (Stimulus :type "AIStimulus Structure"))
  (cast `/Game/AnimStarterPack/Ue4ASP_Character` Actor)
  (`BlackboardComponent.SetValueAsBool` (`AIBlueprintHelperLibrary.GetBlackboard` null) "CanSeePlayer" (`.bSuccessfullySensed` (break `AIStimulus` Stimulus))))

(fn `UserConstructionScript`)